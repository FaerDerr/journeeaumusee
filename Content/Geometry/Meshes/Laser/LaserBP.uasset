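; LaserBP is a laser beam actor that stretches a static mesh to the first surface in front of it.
; Each tick it runs a 2000-unit Visibility line trace along the mesh's forward vector, with one-frame debug drawing left on.
; On a hit it sets the mesh's world X scale directly to the hit distance with a thin cross-section, and on a miss it scales to zero.
; Mesh collision is disabled at BeginPlay.
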(event EventTick
  (params (DeltaSeconds :type Float%20%28single-precision%29))
  (bind _staticmesh (Variables|Default|GetStaticMesh))
  (bind _returnvalue (Transformation|GetWorldLocation _staticmesh))
  (bind (_outhit _returnvalue_2) (Collision|LineTraceByChannel _returnvalue (+ _returnvalue (* (Math|Vector|GetForwardVector _staticmesh) 2e+03)) "TraceTypeQuery1" false 0 "ForOneFrame"))
  (if _returnvalue_2
    (Transformation|SetWorldScale3D (Variables|Default|GetStaticMesh) (Math|Vector|MakeVector (Math|Vector|VectorLength (- (.TraceStart (Collision|BreakHitResult _outhit)) (.ImpactPoint (Collision|BreakHitResult _outhit)))) 0.02 0.02))
    (else
      (Transformation|SetWorldScale3D (Variables|Default|GetStaticMesh) "0, 0, 0"))))

(event EventBeginPlay
  (Collision|SetCollisionEnabled (Variables|Default|GetStaticMesh) "NoCollision"))

(fn ConstructionScript)